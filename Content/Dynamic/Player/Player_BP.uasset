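; Player camera for a map game, with orbit, zoom and pan, plus click detection of UK counties.
; Zoom and held-button mouse rotation set spherical coordinates that place the camera looking back at the actor origin.
; Movement follows camera yaw, adds edge-axis values and is limited by hardcoded bounds.
; Left click converts the cursor hit to map percentages, and BP_GameState samples the map texture's color to identify the county, which is printed.
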(event `self.ReceiveBeginPlay`
  (`self.UpdateCameraLocation&Rotation`))

(event `InputAction|WheelMouseUp`
  (params (Key :type "Key Structure"))
  ;[1 1 1] Zoom
  (:`Pressed`
    (set `self.Camera Radius` (`KismetMathLibrary.FClamp` (- (`self.Camera Radius`) (`self.ZoomSpeed`)) (`self.RadiusMin`) (`self.RadiusMax`)))
    (`self.UpdateCameraLocation&Rotation` :!label _label)))

(event `InputAction|WheelMouseDown`
  (params (Key :type "Key Structure"))
  ;[1 1 1] Zoom
  (:`Pressed`
    (set `self.Camera Radius` (`KismetMathLibrary.FClamp` (+ (`self.Camera Radius`) (`self.ZoomSpeed`)) (`self.RadiusMin`) (`self.RadiusMax`)))
    (goto _label)))

(event `InputAction|RotateCamera`
  (params (Key :type "Key Structure"))
  ;[1 1 1] Rotation
  (:`Pressed`
    (set `self.bRotateCamera?` true))
  (:`Released`
    (set `self.bRotateCamera?` false)))

(event `InputAxis|MouseX`
  (params (AxisValue :type "Float (single-precision)"))
  ;[1 1 1] Rotation
  (if (and (`self.bRotateCamera?`) (`self.bRotationAllowed`))
    (set `self.CAmera Z Angle` (+ (* AxisValue (`self.RotateSpeed`)) (`self.CAmera Z Angle`)))
    (`self.UpdateCameraLocation&Rotation` :!label _label_2)))

(event `InputAxis|MouseY`
  (params (AxisValue :type "Float (single-precision)"))
  ;[1 1 1] Rotation
  (if (and (`self.bRotateCamera?`) (`self.bRotationAllowed`))
    (set `self.Camera Height Angle` (+ (* AxisValue (`self.RotateSpeed`)) (`self.Camera Height Angle`)))
    (goto _label_2)))

(event `InputAxis|MoveForward`
  (params (AxisValue :type "Float (single-precision)"))
  (bind _camera (`self.Camera`))
  (bind (_returnvalue_x _returnvalue_y) (`KismetMathLibrary.BreakVector` (`SceneComponent.K2_GetComponentLocation` _camera)))
  ;[1 1 1] Movimiento
  (`self.MoveUp` (`KismetMathLibrary.GetForwardVector` (`self.Isolate Yaw` (`SceneComponent.K2_GetComponentRotation` _camera))) AxisValue _returnvalue_x))

(event `InputAxis|MoveRight`
  (params (AxisValue :type "Float (single-precision)"))
  (bind _camera (`self.Camera`))
  (bind (_returnvalue_x _returnvalue_y) (`KismetMathLibrary.BreakVector` (`SceneComponent.K2_GetComponentLocation` _camera)))
  ;[1 1 1] Movimiento
  (`self.MoveRight` (`KismetMathLibrary.GetRightVector` (`self.Isolate Yaw` (`SceneComponent.K2_GetComponentRotation` _camera))) AxisValue _returnvalue_y))

(event `InputAction|LeftClick`
  (params (Key :type "Key Structure"))
  (bind (_bblockinghit _binitialoverlap _time _distance _location) (`GameplayStatics.BreakHitResult` (`PlayerController.GetHitResultUnderCursorByChannel` (`GameplayStatics.GetPlayerController` 0) "TraceTypeQuery1" true)))
  (:`Pressed`
    (`KismetSystemLibrary.PrintString` (`KismetStringLibrary.Conv_VectorToString` _location))
    (bind _asbp_game_state (cast `/Game/BP_GameState` (`GameplayStatics.GetGameState`)))
    (bind (_mapsize_x _mapsize_y) (`KismetMathLibrary.BreakVector2D` (`/Game/BP_GameState.MapSize` _asbp_game_state)))
    (bind _returnvalue (`LongLiveTheKingGameState.MapUnitsToPercent` _asbp_game_state (`KismetMathLibrary.FTrunc` (.y _location)) (`KismetMathLibrary.FTrunc` (* (.x _location) -1.0)) (`KismetMathLibrary.MakeVector2D` _mapsize_x _mapsize_y)))
    (bind _returnvalue_2 (`LongLiveTheKingGameState.GetCoordColor` _asbp_game_state _returnvalue "/Game/Static/Map/Tiles/UKMapData.UKMapData"))
    (`|ExecutionSequence`
      (:`then_0`
        (`/Game/BP_GameState.LogColor` _asbp_game_state _returnvalue_2))
      (:`then_1`
        (bind _returnvalue_3 (`LongLiveTheKingGameState.FindCountyByColor` _asbp_game_state _returnvalue_2))
        (`KismetSystemLibrary.PrintString` _returnvalue_3)))))

(fn `IsInBounds`
  (params (AxisAmount :type "Float (double-precision)") (Location :type "Float (double-precision)") (Min :type "Float (double-precision)") (Max :type "Float (double-precision)"))
  (returns (bIsInBounds :type Boolean) (AxisNewAmount :type "Float (double-precision)"))
  (bind _returnvalue (<= AxisAmount 0.0))
  (if (< Location Max)
    (if (> Location Min)
      (return true AxisAmount)
      (elif (not _returnvalue)
        (return false AxisAmount)
        (else
          _)))
    (elif _returnvalue
      (return false AxisAmount)
      (else
        _)))
  (return false 0.0))

(fn `MoveRight`
  (params (Vector :type "Vector Structure") (AxisAmount :type "Float (double-precision)") (Location :type "Float (double-precision)"))
  (bind (_bisinbounds _axisnewamount) (`self.IsInBounds` (+ AxisAmount (`self.EdgeRightAxis`)) Location 28000.0 41000.0))
  (`self.K2_SetActorLocation` (`self.AddVectorToLocation` Vector (* (`KismetMathLibrary.FClamp` _axisnewamount -1.0) (`self.MovementSpeed`)))))

(fn `MoveUp`
  (params (Vector :type "Vector Structure") (AxisAmount :type "Float (double-precision)") (Location :type "Float (double-precision)"))
  (bind (_bisinbounds _axisnewamount) (`self.IsInBounds` (+ AxisAmount (`self.EdgeForwardAxis`)) Location -53000.0 -17000.0))
  (`self.K2_SetActorLocation` (`self.AddVectorToLocation` Vector (* (`KismetMathLibrary.FClamp` _axisnewamount -1.0) (`self.MovementSpeed`)))))

(fn `UpdateCameraLocation&Rotation`
  (`SceneComponent.K2_SetRelativeLocationAndRotation` (`self.Camera`) (`.Location` (`self.PointOnASphere` (`self.Camera Radius`) (`self.CAmera Z Angle`) (`self.Camera Height Angle`))) (`KismetMathLibrary.FindLookAtRotation` (`SceneComponent.RelativeLocation` (`self.Camera`)) (`KismetMathLibrary.MakeVector` 0.0)) false false))

(fn `UserConstructionScript`
  (`self.UpdateCameraLocation&Rotation`))