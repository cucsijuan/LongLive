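; BP_Map is a map actor that pairs a map mesh with a configurable ocean water surface.
; The construction script scales the water mesh on X and Y, creates its dynamic material, then applies scale, variation, wave speed and two colour settings.
; It also stores a dynamic M_Uk_CFG material instance for the map mesh.
; A GetMeshSize helper returns the water surface's X and Y bounds extents.
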(fn `GetMapMaterial`
  (returns (Material :type "MaterialInstanceDynamic Object Reference"))
  (bind _returnvalue (`PrimitiveComponent.CreateDynamicMaterialInstance` (`self.MApMesh`) 0 "/Game/Dynamic/Map/Materials/M_Uk_CFG.M_Uk_CFG"))
  (return _returnvalue))

(fn `GetMeshSize`
  (returns (Size :type "Vector2D Structure"))
  (bind (_origin _boxextent) (`KismetSystemLibrary.GetComponentBounds` (`self.WaterSurface`)))
  (return (`KismetMathLibrary.MakeVector2D` (.x _boxextent) (.y _boxextent))))

(fn `UserConstructionScript`
  (bind _watersurface (`self.WaterSurface`))
  (bind _water_material (`self.Water Material`))
  (bind _returnvalue (`PrimitiveComponent.CreateDynamicMaterialInstance` _watersurface 0 (`self.Ocean Material`)))
  (set `self.Water Material` _returnvalue)
  (`SceneComponent.SetRelativeScale3D` _watersurface (`KismetMathLibrary.MakeVector` (`self.Water Scale X`) (`self.Water Scale Y`) 1.0))
  (`MaterialInstanceDynamic.SetScalarParameterValue` _water_material "Water Scale" (`self.Overall Water Scale`))
  (`MaterialInstanceDynamic.SetScalarParameterValue` _water_material "Variation Amount" (`self.Variation Amount`))
  (`MaterialInstanceDynamic.SetScalarParameterValue` _water_material "Wave Speed" (`self.Wave Speed`))
  (`MaterialInstanceDynamic.SetVectorParameterValue` _water_material "WaterColor A" (`self.Primary Water Color`))
  (`MaterialInstanceDynamic.SetVectorParameterValue` _water_material "WaterColor B" (`self.Secondary Water Color`))
  (bind _material (`self.GetMapMaterial`))
  (set `self.MapMaterial` _material))