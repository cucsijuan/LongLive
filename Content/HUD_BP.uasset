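; HUD Blueprint that detects the cursor at the screen edges and sets edge-movement axes on the owning Player_BP.
; DrawHUD lays out eight input-consuming edge and corner hitboxes each frame, with visible overlays.
; Comma-delimited hitbox names encode type, ID and sub-index, which cursor-over events parse to pick a direction.
; Entering a box sets forward and/or right axes, with corners setting both, and leaving resets both to zero.
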(event `self.ReceiveDrawHUD`
  (params (SizeX :type Integer) (SizeY :type Integer))
  (bind _output_get (set `self.Screen Res` (`KismetMathLibrary.MakeVector2D` (`KismetMathLibrary.Conv_IntToDouble` SizeX) (`KismetMathLibrary.Conv_IntToDouble` SizeY))))
  (`self.DrawEdgeHitboxes` 0 (0.0 0.0) _output_get 32.0 true (struct :`R` 0.177083 :`G` 1.0 :`B` 0.20367 :`A` 1.0) true))

(event `self.ReceiveBeginPlay`
  (bind _asplayer_bp (cast `/Game/Player_BP` (`self.GetOwningPawn`)))
  (set `self.OwningPawn` _asplayer_bp))

(event `self.ReceiveHitBoxBeginCursorOver`
  (params (BoxName :type Name))
  (bind _element_id_s (`self.GetHitBoxType` BoxName)
    (:`EdgeBox`
      (`self.EdgeBoxEvents` _element_id_s
        (:`Top Left`
          (`self.EdgeMovement` :!label _label))
        (:`Top Middle`
          (goto _label :!via `Top Middle`))
        (:`Top Right`
          (goto _label :!via `Top Right`))
        (:`Middle Right`
          (goto _label :!via `Middle Right`))
        (:`Bottom Right`
          (goto _label :!via `Bottom Right`))
        (:`Bottom Middle`
          (goto _label :!via `Bottom Middle`))
        (:`Bottom Left`
          (goto _label :!via `Bottom Left`))
        (:`Middle Left`
          (goto _label :!via `Middle Left`))))))

(event `self.ReceiveHitBoxEndCursorOver`
  (params (BoxName :type Name))
  (bind _element_id_s (`self.GetHitBoxType` BoxName)
    (:`EdgeBox`
      (`self.EdgeBoxEvents` _element_id_s
        (:`Top Left`
          _)
        (:`Top Middle`
          _)
        (:`Top Right`
          _)
        (:`Middle Right`
          _)
        (:`Bottom Right`
          _)
        (:`Bottom Middle`
          _)
        (:`Bottom Left`
          _)
        (:`Middle Left`
          _))
      (`self.ResetEdgeMovement`))))

(fn `Draw Hit Box With Overlay`
  (params (Position :type "Vector2D Structure") (Size :type "Vector2D Structure") (Name :type Name) (`bConsumeInput?` :type Boolean) (Priority :type Integer) (`bShowOverlay?` :type Boolean) (OverlayColour :type "LinearColor Structure"))
  (bind (_x _y) (`KismetMathLibrary.BreakVector2D` Size))
  (bind (_x_2 _y_2) (`KismetMathLibrary.BreakVector2D` Position))
  (`self.AddHitBox` Position Size Name `bConsumeInput?` Priority)
  (if `bShowOverlay?`
    (`self.DrawRect` OverlayColour _x_2 _y_2 _x _y)))

(fn `DrawEdgeHitboxes`
  (params (ID :type Integer) (Location :type "Vector2D Structure") (Size :type "Vector2D Structure") (`Edge Thickness` :type "Float (double-precision)") (`bShowOverlays?` :type Boolean) (OverlayColour :type "LinearColor Structure") (`bConsumeInput?` :type Boolean) (Priority :type Integer))
  (bind _l_edgethickness (`self.L_EdgeThickness`))
  (bind _returnvalue (`KismetMathLibrary.MakeVector2D` _l_edgethickness _l_edgethickness))
  (bind (_x_length _y_length) (`self.CreatEedgeHitBoxSizes` (`self.L_Size`) _l_edgethickness))
  (bind (_top_left _top_middle _top_right _middle_right _bottom_right _bottom_middle _bottom_left _middle_left) (`self.GEt8LocationsForedges` (`self.L_Location`) (`self.L_Size`) (`self.L_EdgeThickness`)))
  (set `self.L_Id` ID)
  (set `self.L_Location` Location)
  (set `self.L_Size` Size)
  (set `self.L_EdgeThickness` `Edge Thickness`)
  (set `self.L_ShowOverlays` `bShowOverlays?`)
  (set `self.L_OverlayColour` OverlayColour)
  (set `self.L_ConsumeInput` `bConsumeInput?`)
  (set `self.L_Priority` Priority)
  (for _index (range 8)
    (`self.Draw Hit Box With Overlay` (select `int` _index :`0` _top_left :`1` _top_middle :`2` _top_right :`3` _middle_right :`4` _bottom_right :`5` _bottom_middle :`6` _bottom_left :`7` _middle_left) (select `int` _index :`0` _returnvalue :`1` _x_length :`2` _returnvalue :`3` _y_length :`4` _returnvalue :`5` _x_length :`6` _returnvalue :`7` _y_length) (`self.CreateHitBoxName` "EdgeBox" (`self.L_Id`) _index) (`self.L_ConsumeInput`) (`self.L_Priority`) (`self.L_ShowOverlays`) (`self.L_OverlayColour`))))

(fn `ResetEdgeMovement`
  (bind _owningpawn (`self.OwningPawn`))
  (set `/Game/Player_BP.EdgeForwardAxis` 0.0 _owningpawn)
  (set `/Game/Player_BP.EdgeRightAxis` 0.0 _owningpawn))

(fn `UserConstructionScript`)